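; EvilBalloon is an enemy physics balloon that moves vertically, cycles its colour through a dynamic material, and destroys itself outside height limits.
; Any hit stops its physics and collision, calling GameOver if it struck the BalloonScrollerCharacter.
; The first hit also triggers an explosion with audio, removes the balloon and TNT components, and radially pushes nearby components.
; Its own GameOver event resets its velocity to a fixed upward drift.
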(event `/Game/BalloonGame/Blueprints/BalloonScrollerObstacle.ReceiveBeginPlay`
  (`PrimitiveComponent.SetPhysicsLinearVelocity` (`self.Sphere1`) (`KismetMathLibrary.MakeVector` 0.0 0.0 (`self.VertSpeed`)) false "None"))

(event `self.ReceiveActorBeginOverlap`
  (params (OtherActor :type "Actor Object Reference")))

(event `/Game/BalloonGame/Blueprints/BalloonScrollerObstacle.ReceiveTick`
  (params (DeltaSeconds :type "Float (single-precision)"))
  (bind _returnvalue (`KismetSystemLibrary.GetGameTimeInSeconds`))
  (bind _z (.z (`SceneComponent.K2_GetComponentLocation` (`self.Sphere1`))))
  (`MaterialInstanceDynamic.SetVectorParameterValue` (`self.BalloonMat_D`) "BalloonColour" (make `LinearColor` (`KismetMathLibrary.Abs` (`KismetMathLibrary.Sin` (/ _returnvalue 0.2))) (`KismetMathLibrary.Abs` (`KismetMathLibrary.Sin` (/ _returnvalue 0.1))) (`KismetMathLibrary.Abs` (`KismetMathLibrary.Cos` (/ _returnvalue 0.3)))))
  (`/Engine/EditorBlueprintResources/StandardMacros.FlipFlop`
    (:`A`
      (if (`self.dead`)
        _
        (elif (<= _z -600.0)
          (`self.K2_DestroyActor` :!label _label)
          (elif (>= _z 500.0)
            (goto _label)))))))

(event `self.ReceiveHit`
  (params (MyComp :type "PrimitiveComponent Object Reference") (Other :type "Actor Object Reference") (OtherComp :type "PrimitiveComponent Object Reference") (bSelfMoved :type Boolean) (HitLocation :type "Vector Structure") (HitNormal :type "Vector Structure") (NormalImpulse :type "Vector Structure") (Hit :type "HitResult Structure (by ref)"))
  (bind _sphere1 (`self.Sphere1`))
  (bind _sphere1_2 (`self.Sphere1`))
  (bind _returnvalue (`SceneComponent.K2_GetComponentLocation` _sphere1_2))
  (`PrimitiveComponent.SetSimulatePhysics` _sphere1 false)
  (`PrimitiveComponent.SetCollisionEnabled` _sphere1 "NoCollision")
  (bind _asballoon_scroller_character (cast `/Game/BalloonGame/Blueprints/BalloonScrollerCharacter` Other)
    (:`then`
      (`/Game/BalloonGame/Blueprints/BalloonScrollerCharacter.GameOver` _asballoon_scroller_character))
    (:`CastFailed`
      _))
  (set `self.HitLoc` HitLocation)
  (set `self.HitNorm` HitNormal)
  (if (not (`self.dead`))
    (set `self.dead` true)
    (`ActorComponent.Activate` (`self.Explode`) true)
    (`KismetSystemLibrary.Delay` 0.1)
    (`AddComponent|AudioComponent_1` :`RelativeTransform` (`SceneComponent.GetRelativeTransform` (`self.ballon`)))
    (`ActorComponent.K2_DestroyComponent` (`self.ballon`))
    (`ActorComponent.K2_DestroyComponent` (`self.TNT`))
    (bind _outcomponents (`KismetSystemLibrary.SphereOverlapComponents_NEW` _returnvalue 200.0 (`self.ExpAffects`)))
    (`PrimitiveComponent.AddRadialImpulse` _outcomponents _returnvalue 200.0 100000.0 "RIF_Constant" false)
    (`SceneComponent.SetRelativeScale3D` _sphere1_2 (0.3 0.3 0.3))
    (`KismetSystemLibrary.Delay` 1.0)
    (set `self.bAutoDestroyWhenFinished` true)))

(event `GameOver`
  (`PrimitiveComponent.SetPhysicsLinearVelocity` (`self.Sphere1`) (0.0 0.0 50.0) false "None"))

(fn `UserConstructionScript`
  (bind _returnvalue (`PrimitiveComponent.CreateDynamicMaterialInstance` (`self.ballon`) 0 "/Game/BalloonGame/Materials/EnemyBalloonDynamic.EnemyBalloonDynamic"))
  (set `self.BalloonMat_D` _returnvalue))