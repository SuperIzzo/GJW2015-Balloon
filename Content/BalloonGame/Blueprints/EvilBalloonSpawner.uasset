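; Spawner actor for the balloon game that keeps creating EvilBalloon obstacles at random intervals.
; Tick counts down a timer, resets it to a random one-to-two-second delay and spawns a balloon at a random X along a fixed low Z line in world space.
; BeginPlay also plays BallSpawnFrequency, but the spawn logic does not read it.
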(event `/Game/BalloonGame/Blueprints/BalloonObstacleSpawner.ReceiveBeginPlay`
  (`Timeline|Ball spawn frequency`))

(event `self.ReceiveActorBeginOverlap`
  (params (OtherActor :type "Actor Object Reference")))

(event `/Game/BalloonGame/Blueprints/BalloonObstacleSpawner.ReceiveTick`
  (params (DeltaSeconds :type "Float (single-precision)"))
  (bind _newobstacletimer (`self.NewObstacleTimer`))
  (set `self.NewObstacleTimer` (- _newobstacletimer DeltaSeconds))
  (if (<= _newobstacletimer 0.0)
    (set `self.NewObstacleTimer` (+ (`KismetMathLibrary.RandomFloat`) 1.0))
    (`|SpawnActorFromClass` "/Game/BalloonGame/Blueprints/EvilBalloon.EvilBalloon_C" (`KismetMathLibrary.MakeTransform` (`KismetMathLibrary.MakeVector` (* (- (`KismetMathLibrary.RandomFloat`) 0.5) 800.0) 0.0 -500.0) (`KismetMathLibrary.MakeRotator` 0.0) (`KismetMathLibrary.MakeVector` 1.0 1.0 1.0)) "Undefined" "OverrideRootScale")))

(fn `UserConstructionScript`)