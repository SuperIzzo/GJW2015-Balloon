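; Endlessly scrolling, randomly winding well for the balloon game, built from spline meshes.
; Construction seeds a straight spline; Tick moves it downward and, after each TotalMovement of travel, appends a randomly X-offset point and a new mesh segment.
; Segments trail the newest point by one, and every BalloonScrollerGameArea receives the previous offset as WallNextPoint.
; Old points and meshes are never removed.
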(event `/Game/BalloonGame/Blueprints/BalloonScrollerCharacter.ReceiveBeginPlay`)

(event `self.ReceiveActorBeginOverlap`
  (params (OtherActor :type "Actor Object Reference")))

(event `/Game/BalloonGame/Blueprints/BalloonScrollerCharacter.ReceiveTick`
  (params (DeltaSeconds :type "Float (single-precision)"))
  (bind _returnvalue (`KismetMathLibrary.RandomFloat`))
  (bind _totalmovement (`self.totalMovement`))
  (bind _curmove (`self.curMove`))
  (bind _spline (`self.Spline`))
  (bind _returnvalue_2 (`SplineComponent.GetNumberOfSplinePoints` _spline))
  (bind _returnvalue_3 (* (/ DeltaSeconds (`self.moveSecs`)) _totalmovement))
  (bind (_location _tangent) (`SplineComponent.GetLocationAndTangentAtSplinePoint` _spline (- _returnvalue_2 2) "Local"))
  (bind (_location_2 _tangent_2) (`SplineComponent.GetLocationAndTangentAtSplinePoint` _spline (- _returnvalue_2 3) "Local"))
  (set `self.curMove` (+ (`self.curMove`) _returnvalue_3))
  (`SceneComponent.K2_AddWorldOffset` (`self.Spline`) (`KismetMathLibrary.MakeVector` 0.0 0.0 (* _returnvalue_3 -1.0)) true false)
  (if (>= _curmove _totalmovement)
    (set `self.curMove` (- _curmove _totalmovement))
    (bind _output_get (set `self.CurSegW` (* (- _returnvalue 0.5) 300.0)))
    (`SplineComponent.AddSplinePoint` _spline (`KismetMathLibrary.MakeVector` _output_get _returnvalue 3000.0) "World")
    (bind _returnvalue_4 (`AddComponent|Spline Mesh Component_3980`))
    (`SplineMeshComponent.SetSplineUpDir` _returnvalue_4 (`KismetMathLibrary.RotateAngleAxis` _tangent_2 -90.0 (0.0 10.0 0.0)))
    (`SplineMeshComponent.SetStartAndEnd` _returnvalue_4 _location_2 (* _tangent_2 1.0) (* _location 1.0) _tangent)
    (`SceneComponent.K2_AttachTo` _returnvalue_4 _spline "None" "KeepRelativeOffset" true)
    (bind _outactors (`GameplayStatics.GetAllActorsOfClass` "/Game/BalloonGame/Blueprints/BalloonScrollerGameArea.BalloonScrollerGameArea_C"))
    (for _array_element _outactors
      (set `/Game/BalloonGame/Blueprints/BalloonScrollerGameArea.WallNextPoint` (`self.PrevSegW`) _array_element))
    (set `self.PrevSegW` (`self.CurSegW`))))

(fn `UserConstructionScript`
  (bind _spline (`self.Spline`))
  (bind _returnvalue (`SplineComponent.GetNumberOfSplinePoints` _spline))
  (bind (_location _tangent) (`SplineComponent.GetLocationAndTangentAtSplinePoint` _spline (- _returnvalue 1) "Local"))
  (bind (_location_2 _tangent_2) (`SplineComponent.GetLocationAndTangentAtSplinePoint` _spline (- _returnvalue 2) "Local"))
  (`SplineComponent.SetLocationAtSplinePoint` _spline 0 (`KismetMathLibrary.MakeVector` 0.0 0.0 -1000.0) "Local")
  (`SplineComponent.SetLocationAtSplinePoint` _spline 1 (`KismetMathLibrary.MakeVector` 0.0) "Local")
  (for _index (range 1 3)
    (`SplineComponent.AddSplinePoint` _spline (`KismetMathLibrary.MakeVector` 0.0 0.0 (* _index 1000.0)) "World")
    (bind _returnvalue_2 (`AddComponent|SplineMeshComponent_481`))
    (`SplineMeshComponent.SetSplineUpDir` _returnvalue_2 (`KismetMathLibrary.RotateAngleAxis` _tangent_2 -90.0 (0.0 10.0 0.0)))
    (`SplineMeshComponent.SetStartAndEnd` _returnvalue_2 _location_2 _tangent_2 _location _tangent)
    (`SceneComponent.K2_AttachTo` _returnvalue_2 _spline "None" "KeepRelativeOffset" true))
  (`SplineComponent.AddSplinePoint` _spline (`KismetMathLibrary.MakeVector` 0.0 0.0 3000.0) "World"))