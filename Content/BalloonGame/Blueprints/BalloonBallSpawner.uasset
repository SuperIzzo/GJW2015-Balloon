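; Spawner actor for the balloon game that periodically creates BalloonScrollerBall obstacles.
; Tick counts down a timer and, when it expires, resets it to a random interval of up to two seconds.
; Each ball spawns at a fixed height with a random horizontal X offset centered on the world origin, independent of the spawner's own position.
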(event `self.ReceiveBeginPlay`)

(event `self.ReceiveActorBeginOverlap`
  (params (OtherActor :type "Actor Object Reference")))

(event `/Game/BalloonGame/Blueprints/BalloonObstacleSpawner.ReceiveTick`
  (params (DeltaSeconds :type "Float (single-precision)"))
  (bind _newobstacletimer (`self.NewObstacleTimer`))
  (set `self.NewObstacleTimer` (- _newobstacletimer DeltaSeconds))
  (if (<= _newobstacletimer 0.0)
    (set `self.NewObstacleTimer` (* (`KismetMathLibrary.RandomFloat`) 2.0))
    (`|SpawnActorFromClass` "/Game/BalloonGame/Blueprints/BalloonScrollerBall.BalloonScrollerBall_C" (`KismetMathLibrary.MakeTransform` (`KismetMathLibrary.MakeVector` (* (- (`KismetMathLibrary.RandomFloat`) 0.5) 850.0) 0.0 400.0) (struct) (1.0 1.0 1.0)) "Undefined" "OverrideRootScale")))

(fn `UserConstructionScript`)