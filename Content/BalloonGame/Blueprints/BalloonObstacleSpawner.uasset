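; Balloon minigame spawner actor that creates scrolling obstacles at random intervals.
; Tick counts down a timer, and when it expires resets it to a random delay of up to two seconds and spawns a BalloonScrollerObstacle.
; Each obstacle appears at a fixed height with randomized horizontal position, pitch tilt and width scale, placed in world space independent of the spawner's own transform.
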(event `self.ReceiveBeginPlay`)

(event `self.ReceiveActorBeginOverlap`
  (params (OtherActor :type "Actor Object Reference")))

(event `self.ReceiveTick`
  (params (DeltaSeconds :type "Float (single-precision)"))
  (bind _newobstacletimer (`self.NewObstacleTimer`))
  (set `self.NewObstacleTimer` (- _newobstacletimer DeltaSeconds))
  (if (<= _newobstacletimer 0.0)
    (set `self.NewObstacleTimer` (* (`KismetMathLibrary.RandomFloat`) 2.0))
    (`|SpawnActorFromClass` "/Game/BalloonGame/Blueprints/BalloonScrollerObstacle.BalloonScrollerObstacle_C" (`KismetMathLibrary.MakeTransform` (`KismetMathLibrary.MakeVector` (* (- (`KismetMathLibrary.RandomFloat`) 0.5) 850.0) 0.0 400.0) (`KismetMathLibrary.MakeRotator` 0.0 (* (- (`KismetMathLibrary.RandomFloat`) 0.5) 45.0)) (`KismetMathLibrary.MakeVector` (+ (* (`KismetMathLibrary.RandomFloat`) 1.2) 0.5) 1.0 1.0)) "Undefined" "OverrideRootScale")))

(fn `UserConstructionScript`)