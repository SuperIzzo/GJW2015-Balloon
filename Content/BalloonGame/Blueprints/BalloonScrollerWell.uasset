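; Scrolling well actor for the balloon game that moves its wall segment vertically to create looping motion.
; Tick advances a normalized wall position into an interpolated Z location, wrapping it each cycle until the game is won.
; Staged delays at BeginPlay remove the Sh pieces, with ShA's initial visibility and collision set by StartWithShield.
; Character dispatchers raise the movement scale on player death, or stop wrapping and hide a mesh on a win.
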(event `self.ReceiveBeginPlay`
  (bind _asballoon_scroller_character (cast `/Game/BalloonGame/Blueprints/BalloonScrollerCharacter` (`GameplayStatics.GetPlayerPawn` 0)))
  (add `/Game/BalloonGame/Blueprints/BalloonScrollerCharacter.PlayerStatus` _asballoon_scroller_character (delegate `PayerDied`))
  (add `/Game/BalloonGame/Blueprints/BalloonScrollerCharacter.Debug` _asballoon_scroller_character (delegate `WinGame`))
  (`KismetSystemLibrary.Delay` 1.0)
  (`ActorComponent.K2_DestroyComponent` (`self.ShC1`))
  (`ActorComponent.K2_DestroyComponent` (`self.ShC2`))
  (`KismetSystemLibrary.Delay` 0.5)
  (`ActorComponent.K2_DestroyComponent` (`self.ShB1`))
  (`ActorComponent.K2_DestroyComponent` (`self.ShB2`))
  (`KismetSystemLibrary.Delay` 0.5)
  (`ActorComponent.K2_DestroyComponent` (`self.ShA`)))

(event `self.ReceiveTick`
  (params (DeltaSeconds :type "Float (single-precision)"))
  (bind _wallpos (`self.WallPos`))
  (bind _totalmovement (`self.totalMovement`))
  (bind _well_seg0 (`self.Well_Seg0`))
  (bind _returnvalue (* DeltaSeconds (`self.TimeScale`)))
  (if (>= _wallpos 1.0)
    (if (not (`self.GameWon`))
      (`SceneComponent.K2_AddWorldOffset` _well_seg0 (`KismetMathLibrary.MakeVector` 0.0 0.0 (* _wallpos _totalmovement -1.0 (`self.MoveScale`))) false true)
      (set `self.WallPos` (- _wallpos 1.0))))
  (set `self.WallPos` (+ _returnvalue _wallpos))
  (`SceneComponent.K2_SetWorldLocation` _well_seg0 (`KismetMathLibrary.MakeVector` 0.0 0.0 (* (`KismetMathLibrary.FInterpTo` (* _wallpos _totalmovement) _totalmovement _returnvalue 0.01) (`self.MoveScale`))) false false))

(event `PayerDied`
  (set `self.MoveScale` 2.0))

(event `WinGame`
  (set `self.GameWon` true)
  (`SceneComponent.SetVisibility` (`self.StaticMesh14`) false false))

(fn `UserConstructionScript`
  (bind _sha (`self.ShA`))
  (`SceneComponent.SetVisibility` _sha (`self.StartWithShield`) true)
  (`PrimitiveComponent.SetCollisionEnabled` _sha (select `bool` (`self.StartWithShield`) :`false` "QueryAndPhysics" :`true` "NoCollision" :!type "ECollisionEnabled Enum")))