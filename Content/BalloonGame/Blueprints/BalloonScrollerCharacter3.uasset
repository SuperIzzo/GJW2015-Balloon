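; Player balloon pawn for the balloon scroller, pushed along X and Z by input impulses on its physics Sphere.
; The Power input fires a cooldown-gated radial impulse at nearby objects with a brief light flash.
; GameOver swaps the sphere and light for a destructible shattered at the last hit point, blasts nearby objects and sets the game mode's scroll speed to FallSpeed.
; It then notifies balls and obstacles and loads the main menu after a delay.
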(event `/Game/BalloonGame/Blueprints/BalloonScrollerCharacter.ReceiveBeginPlay`
  (set `self.AbilityNextuse` (- (`GameplayStatics.GetRealTimeSeconds`) (`self.AbilityCooldown`))))

(event `/Game/BalloonGame/Blueprints/BalloonScrollerCharacter.ReceiveActorBeginOverlap`
  (params (OtherActor :type "Actor Object Reference")))

(event `/Game/BalloonGame/Blueprints/BalloonScrollerCharacter.ReceiveTick`
  (params (DeltaSeconds :type "Float (single-precision)")))

(event `GameOver`
  (bind _sphere (`self.Sphere`))
  (bind _returnvalue (`SceneComponent.GetRelativeTransform` _sphere))
  (if (not (`self.Dead`))
    (set `self.Dead` true)
    (`self.PlayerStatus`)
    (`KismetSystemLibrary.Delay` 0.02)
    (bind _returnvalue_2 (`AddComponent|Destructible Component_6` :`RelativeTransform` _returnvalue))
    (`AddComponent|Audio Component_3` :`RelativeTransform` _returnvalue)
    (`ActorComponent.K2_DestroyComponent` _sphere)
    (`ActorComponent.K2_DestroyComponent` (`self.PointLight`))
    (bind _asballoon_scroller_game_mode (cast `/Game/BalloonGame/Blueprints/BalloonScrollerGameMode` (`GameplayStatics.GetGameMode`)))
    (set `/Game/BalloonGame/Blueprints/BalloonScrollerGameMode.ScrollSpeed` (`self.FallSpeed`) _asballoon_scroller_game_mode)
    (`PrimitiveComponent.SetMaterial` _returnvalue_2 0 "/Game/BalloonGame/Materials/ShinyBalloonTess_2s.ShinyBalloonTess_2s")
    (`DestructibleComponent.ApplyDamage` _returnvalue_2 50.0 (`self.HitLoc`) (`self.HitNorm`) 500.0)
    (bind _returnvalue_3 (`SceneComponent.K2_GetComponentLocation` _returnvalue_2))
    (bind _outcomponents (`KismetSystemLibrary.SphereOverlapComponents_NEW` _returnvalue_3 400.0 (`self.ExpAffects`)))
    (`PrimitiveComponent.AddRadialImpulse` _outcomponents _returnvalue_3 400.0 500000.0 "RIF_Constant" false)
    (`SceneComponent.SetRelativeScale3D` _returnvalue_2 (0.3 0.3 0.3))
    (bind _outactors (`GameplayStatics.GetAllActorsOfClass` "/Game/BalloonGame/Blueprints/BalloonScrollerBall.BalloonScrollerBall_C"))
    (for _array_element _outactors
      (`/Game/BalloonGame/Blueprints/BalloonScrollerBall.GameOver` _array_element)
      (`KismetSystemLibrary.Delay` 2.5 :!label _label)
      (`GameplayStatics.OpenLevel` "MainMenuLevel"))
    (bind _outactors_2 (`GameplayStatics.GetAllActorsOfClass` "/Game/BalloonGame/Blueprints/BalloonScrollerObstacle.BalloonScrollerObstacle_C"))
    (for _array_element_2 _outactors_2
      (`/Game/BalloonGame/Blueprints/BalloonScrollerObstacle.GameOver` _array_element_2)
      (goto _label))))

(event `self.ReceiveHit`
  (params (MyComp :type "PrimitiveComponent Object Reference") (Other :type "Actor Object Reference") (OtherComp :type "PrimitiveComponent Object Reference") (bSelfMoved :type Boolean) (HitLocation :type "Vector Structure") (HitNormal :type "Vector Structure") (NormalImpulse :type "Vector Structure") (Hit :type "HitResult Structure (by ref)"))
  (set `self.HitLoc` HitLocation)
  (set `self.HitNorm` HitNormal))

(event `InputAxis|MoveRight`
  (params (AxisValue :type "Float (single-precision)"))
  (if (not (`self.Dead`))
    (`PrimitiveComponent.AddImpulse` (`self.Sphere`) (`KismetMathLibrary.MakeVector` (* AxisValue (`self.AccelRate`))) "None" false)))

(event `InputAxis|MoveUp`
  (params (AxisValue :type "Float (single-precision)"))
  (if (not (`self.Dead`))
    (`PrimitiveComponent.AddImpulse` (`self.Sphere`) (`KismetMathLibrary.MakeVector` 0.0 0.0 (* AxisValue (`self.AccelRate`))) "None" false)))

(event `InputAction|Power`
  (params (Key :type "Key Structure" :default "AnyKey"))
  (bind _returnvalue (`GameplayStatics.GetRealTimeSeconds`))
  (bind _dead (`self.Dead`))
  (bind _pointlight (`self.PointLight`))
  (bind _returnvalue_2 (`SceneComponent.K2_GetComponentLocation` (`self.Sphere`)))
  (:`Pressed`
    (if (>= _returnvalue (`self.AbilityNextuse`))
      (if (not _dead)
        (set `self.AbilityNextuse` (+ _returnvalue (`self.AbilityCooldown`)))
        (bind _outcomponents (`KismetSystemLibrary.SphereOverlapComponents_NEW` _returnvalue_2 300.0 (`self.ExpAffects`)))
        (`PrimitiveComponent.AddRadialImpulse` _outcomponents _returnvalue_2 200.0 100000.0 "RIF_Constant" false)
        (`LightComponent.SetIntensity` _pointlight 2000000.0)
        (`KismetSystemLibrary.Delay` 0.4)
        (if (not _dead)
          (`LightComponent.SetIntensity` _pointlight 2000.0))))))

(event `InputAction|ForceQuit`
  (params (Key :type "Key Structure" :default "AnyKey"))
  (:`Pressed`
    (`KismetSystemLibrary.QuitGame` null "Quit")))

(fn `UserConstructionScript`)