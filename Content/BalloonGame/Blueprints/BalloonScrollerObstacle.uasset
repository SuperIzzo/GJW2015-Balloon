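; BalloonScrollerObstacle is a physics-driven obstacle for the balloon scroller game that ends the game when it hits the player.
; It starts moving downward, and Tick uses nested FlipFlops to alternate, on every other frame, between a vertical bounds check that destroys it and a downward impulse.
; A hit on BalloonScrollerCharacter calls that character's GameOver.
; The obstacle's own GameOver event sends it moving upward.
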(event `self.ReceiveBeginPlay`
  (`PrimitiveComponent.SetPhysicsLinearVelocity` (`self.Cube`) (0.0 0.0 -50.0) false "None"))

(event `self.ReceiveActorBeginOverlap`
  (params (OtherActor :type "Actor Object Reference")))

(event `self.ReceiveTick`
  (params (DeltaSeconds :type "Float (single-precision)"))
  (bind _cube (`self.Cube`))
  (bind _z (.z (`SceneComponent.K2_GetComponentLocation` _cube)))
  (`/Engine/EditorBlueprintResources/StandardMacros.FlipFlop`
    (:`A`
      (`/Engine/EditorBlueprintResources/StandardMacros.FlipFlop`
        (:`A`
          (if (<= _z -500.0)
            (`self.K2_DestroyActor` :!label _label)
            (elif (>= _z 500.0)
              (goto _label))))
        (:`B`
          (`PrimitiveComponent.AddImpulse` _cube (0.0 0.0 -500.0) "None" false))))))

(event `self.ReceiveHit`
  (params (MyComp :type "PrimitiveComponent Object Reference") (Other :type "Actor Object Reference") (OtherComp :type "PrimitiveComponent Object Reference") (bSelfMoved :type Boolean) (HitLocation :type "Vector Structure") (HitNormal :type "Vector Structure") (NormalImpulse :type "Vector Structure") (Hit :type "HitResult Structure (by ref)"))
  (bind _asballoon_scroller_character (cast `/Game/BalloonGame/Blueprints/BalloonScrollerCharacter` Other))
  (`/Game/BalloonGame/Blueprints/BalloonScrollerCharacter.GameOver` _asballoon_scroller_character))

(event `GameOver`
  (`PrimitiveComponent.SetPhysicsLinearVelocity` (`self.Cube`) (0.0 0.0 100.0) false "None"))

(fn `UserConstructionScript`)