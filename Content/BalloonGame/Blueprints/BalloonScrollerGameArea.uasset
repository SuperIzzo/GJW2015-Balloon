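; BalloonScrollerGameArea is the game area actor for a balloon scroller game, with a staged component removal at start.
; BeginPlay destroys three groups of components in timed steps: the ShC pair, then the ShB pair, then ShA.
; Tick is empty, and a disconnected chain holds unused looping vertical scroll logic that takes its speed from BalloonScrollerGameMode.
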(event `/Game/BalloonGame/Blueprints/BalloonScrollerCharacter.ReceiveBeginPlay`
  (`KismetSystemLibrary.Delay` 1.0)
  (`ActorComponent.K2_DestroyComponent` (`self.ShC1`))
  (`ActorComponent.K2_DestroyComponent` (`self.ShC2`))
  (`KismetSystemLibrary.Delay` 0.5)
  (`ActorComponent.K2_DestroyComponent` (`self.ShB1`))
  (`ActorComponent.K2_DestroyComponent` (`self.ShB2`))
  (`KismetSystemLibrary.Delay` 0.5)
  (`ActorComponent.K2_DestroyComponent` (`self.ShA`)))

(event `self.ReceiveActorBeginOverlap`
  (params (OtherActor :type "Actor Object Reference")))

(event `/Game/BalloonGame/Blueprints/BalloonScrollerCharacter.ReceiveTick`
  (params (DeltaSeconds :type "Float (single-precision)")))

(fn `UserConstructionScript`)