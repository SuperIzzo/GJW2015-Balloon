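; Game mode for the balloon scroller game that sets up the HUD and announces the game start.
; BeginPlay creates the HUD widget, adds it to the viewport, then binds to and immediately calls its GameStarted dispatcher.
; The bound event starts a GameDuration delay with nothing wired after it, so no end-of-game logic exists here.
; Tick is empty, and a nested FlipFlop debug print of ScrollSpeed is left disconnected.
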(event `GameStarted_Event`
  (`KismetSystemLibrary.Delay` (`self.GameDuration`)))

(event `self.ReceiveBeginPlay`
  (bind _returnvalue (`|CreateWidget` "/Game/BalloonGame/HUD.HUD_C"))
  (`UserWidget.AddToViewport` _returnvalue 0)
  (add `self.GameStarted` (delegate `GameStarted_Event`))
  (`self.GameStarted`))

(event `self.ReceiveTick`
  (params (DeltaSeconds :type "Float (single-precision)")))

(fn `UserConstructionScript`)